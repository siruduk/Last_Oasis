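; Player character Blueprint handling item pickup, spear combat, a UI toggle and storm visuals.
; Capsule overlaps store nearby interactives or LaboA/LaboB actors (end overlap doesn't clear them); F transfers their items to InventoryManager.
; GAS events start stat reduction with a night tag, or reveal the spear with an attack tag; three weapon ranges fill HitList and fire Niagara.
; ToggleStorm switches dust visibility and height fog density.
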(event `Key|Z`
  (params (Key :type "Key Structure"))
  (bind _newvar (`self.NewVar`))
  (:`Pressed`
    (if (`|EnumEquality` (`Widget.Visibility` _newvar) "Visible") :!label _label
      (`Widget.SetVisibility` _newvar "Hidden")
      (else
        (`Widget.SetVisibility` _newvar "Visible")))))

(event `Key|Escape`
  (params (Key :type "Key Structure"))
  (:`Pressed`
    (goto _label)))

(event `self.ReceiveBeginPlay`
  (`ActorComponent.SetActive` (`self.Dust`) false false))

(event `self.StartReduceStat`
  (`AbilitySystemComponent.TryActivateAbilityByClass` (`AbilitySystemBlueprintLibrary.GetAbilitySystemComponent` null) "/Game/Siru/BP/GameplayAbility/GameplayAbility/BPGA_StatReducion.BPGA_StatReducion_C" true)
  (`AbilitySystemBlueprintLibrary.AddLooseGameplayTags` self (`BlueprintGameplayTagLibrary.MakeGameplayTagContainerFromTag` (struct :`TagName` "Game.Night"))))

(event `Key|F`
  (params (Key :type "Key Structure"))
  (bind _inventorymanager (`self.InventoryManager`))
  (bind _interactive_actor (`self.Interactive Actor`))
  (bind _roboactor (`self.RoboActor`))
  (:`Pressed`
    (`/Engine/EditorBlueprintResources/StandardMacros.IsValid` _interactive_actor
      (:`Is Valid`
        (`InventoryManager.GetItem` (`self.InventoryManager`) _interactive_actor)
        (`self.K2_DestroyActor` _interactive_actor))
      (:`Is Not Valid`
        (`KismetSystemLibrary.PrintString` "Can't find interactive")
        (`/Engine/EditorBlueprintResources/StandardMacros.IsValid` _roboactor
          (:`Is Valid`
            (bind _aslabo_a (cast `/Game/Fab/LaboA` _roboactor)
              (:`then`
                (bind _acquired_item (`/Game/Fab/LaboA.Acquired Item` _aslabo_a))
                (`InventoryManager.GetDropItemData` _inventorymanager _acquired_item)
                (`KismetArrayLibrary.Array_Clear` _acquired_item))
              (:`CastFailed`
                (bind _aslabo_b (cast `/Game/Fab/LaboB` _roboactor))
                (bind _acquired_items (`/Game/Fab/LaboB.Acquired Items` _aslabo_b))
                (`InventoryManager.GetDropItemData` _inventorymanager _acquired_items)
                (`KismetArrayLibrary.Array_Clear` _acquired_items)))))))))

(event `self.CapsuleComponent.OnComponentBeginOverlap`
  (params (OverlappedComponent :type "PrimitiveComponent Object Reference") (OtherActor :type "Actor Object Reference") (OtherComp :type "PrimitiveComponent Object Reference") (OtherBodyIndex :type Integer) (bFromSweep :type Boolean) (SweepResult :type "HitResult Structure (by ref)"))
  (bind _asinteractive_actor (cast `InteractiveActor` OtherActor)
    (:`then`
      (set `self.Interactive Actor` _asinteractive_actor))
    (:`CastFailed`
      (bind _aslabo_a (cast `/Game/Fab/LaboA` OtherActor)
        (:`then`
          (set `self.RoboActor` _aslabo_a))
        (:`CastFailed`
          (bind _aslabo_b (cast `/Game/Fab/LaboB` OtherActor))
          (set `self.RoboActor` _aslabo_b))))))

(event `self.CapsuleComponent.OnComponentEndOverlap`
  (params (OverlappedComponent :type "PrimitiveComponent Object Reference") (OtherActor :type "Actor Object Reference") (OtherComp :type "PrimitiveComponent Object Reference") (OtherBodyIndex :type Integer))
  (bind _asinteractive_actor (cast `InteractiveActor` OtherActor)
    (:`then`
      (set `self.Interactive Actor` _asinteractive_actor))
    (:`CastFailed`
      (bind _aslabo_a (cast `/Game/Fab/LaboA` OtherActor)
        (:`then`
          (set `self.RoboActor` _aslabo_a))
        (:`CastFailed`
          (bind _aslabo_b (cast `/Game/Fab/LaboB` OtherActor))
          (set `self.RoboActor` _aslabo_b))))))

(event `self.GetWeapon`
  (`SceneComponent.SetVisibility` (`self.Spear`) true false)
  (`AbilitySystemBlueprintLibrary.AddLooseGameplayTags` self (`BlueprintGameplayTagLibrary.MakeLiteralGameplayTagContainer` (struct :`GameplayTags` (struct :`(TagName` "State.CanAttack"))))))

(event `self.WeaponRange1.OnComponentBeginOverlap`
  (params (OverlappedComponent :type "PrimitiveComponent Object Reference") (OtherActor :type "Actor Object Reference") (OtherComp :type "PrimitiveComponent Object Reference") (OtherBodyIndex :type Integer) (bFromSweep :type Boolean) (SweepResult :type "HitResult Structure (by ref)"))
  (bind _asenemy_ch (cast `EnemyCh` OtherActor))
  (`BlueprintSetLibrary.Set_Add` (`self.HitList`) _asenemy_ch)
  (`ActorComponent.Activate` (`self.Niagara`) true))

(event `self.WeaponRange2.OnComponentBeginOverlap`
  (params (OverlappedComponent :type "PrimitiveComponent Object Reference") (OtherActor :type "Actor Object Reference") (OtherComp :type "PrimitiveComponent Object Reference") (OtherBodyIndex :type Integer) (bFromSweep :type Boolean) (SweepResult :type "HitResult Structure (by ref)"))
  (bind _asenemy_ch (cast `EnemyCh` OtherActor))
  (`BlueprintSetLibrary.Set_Add` (`self.HitList`) _asenemy_ch)
  (`ActorComponent.Activate` (`self.Niagara`) true))

(event `self.WeaponRange3.OnComponentBeginOverlap`
  (params (OverlappedComponent :type "PrimitiveComponent Object Reference") (OtherActor :type "Actor Object Reference") (OtherComp :type "PrimitiveComponent Object Reference") (OtherBodyIndex :type Integer) (bFromSweep :type Boolean) (SweepResult :type "HitResult Structure (by ref)"))
  (bind _asenemy_ch (cast `EnemyCh` OtherActor))
  (`BlueprintSetLibrary.Set_Add` (`self.HitList`) _asenemy_ch)
  (`ActorComponent.Activate` (`self.Niagara`) true))

(fn `ToggleStorm`
  (params (NewParam :type Boolean))
  (`KismetSystemLibrary.PrintString` "ToggleStorm")
  (`SceneComponent.SetVisibility` (`self.Dust`) NewParam false)
  (bind _returnvalue (`GameplayStatics.GetActorOfClass` "/Script/Engine.ExponentialHeightFog"))
  (if (`KismetSystemLibrary.IsValid` _returnvalue)
    (if NewParam
      (bind _component (`ExponentialHeightFog.Component` _returnvalue))
      (`ExponentialHeightFogComponent.SetFogDensity` _component 2.0)
      (else
        (`ExponentialHeightFogComponent.SetFogDensity` _component 0.05)))))

(fn `UserConstructionScript`)