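; BP_Groot is an enemy AI character with a camera-facing health bar and a leaf projectile attack.
; Tick sets chase and attack states by player distance, and at zero HP disables collision, decrements the player's enemy count and destroys it after a delay.
; Sync functions mirror state into ABP_Groot and the Blackboard, with chase state also setting walk speed.
; MagicalLeaf fires BP_LeafBullets outward from three leaf points.
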(event `self.ReceiveBeginPlay`
  (set `self.GoalPos` (`NavigationSystemV1.K2_GetRandomReachablePointInRadius` (`self.K2_GetActorLocation`) 600.0 null null))
  (bind _output_get (set `self.MaxHP` 80.0))
  (set `self.HP` _output_get)
  (set `self.AttackRange` 400.0)
  (set `self.ChaseRange` 800.0)
  (`self.Sync_bCanAttack` true true)
  (`self.Sync_bIsDead` true true)
  (`self.Sync_StateIdx` true true)
  (`KismetArrayLibrary.Array_Clear` (`self.Leaves`))
  (set `self.Leaves` (`|MakeArray` (`self.Leaf1`) (`self.Leaf2`) (`self.Leaf3`)))
  (bind _aswbp_enemy_health (cast `/Game/_shuby/UIs/WBP_EnemyHealth` (`WidgetComponent.GetWidget` (`self.HealthBar`))))
  (bind _healthpbar (`/Game/_shuby/UIs/WBP_EnemyHealth.HealthPBar` _aswbp_enemy_health))
  (bind _output_get_2 (set `self.Health PBar` _healthpbar))
  (`ProgressBar.SetPercent` _healthpbar 1.0)
  (`ProgressBar.SetPercent` _output_get_2 1.0))

(event `self.ReceiveTick`
  (params (DeltaSeconds :type "Float (single-precision)"))
  (bind _returnvalue (`GameplayStatics.GetPlayerCharacter` 0))
  (bind _healthbar (`self.HealthBar`))
  (bind _returnvalue_2 (`KismetMathLibrary.Vector_Distance` (`self.K2_GetActorLocation`) (`self.K2_GetActorLocation` _returnvalue)))
  (if (`GameplayTagAssetInterface.HasMatchingGameplayTag` (`AbilitySystemBlueprintLibrary.GetAbilitySystemComponent` (`GameplayStatics.GetPlayerCharacter` 0)) (struct :`TagName` "State.Dead"))
    (`self.Sync_bCanAttack` true true)
    (`self.Sync_StateIdx` true true))
  (`SceneComponent.K2_SetWorldRotation` _healthbar (`KismetMathLibrary.FindLookAtRotation` (`SceneComponent.K2_GetComponentLocation` _healthbar) (`SceneComponent.K2_GetComponentLocation` (`Actor.RootComponent` (`GameplayStatics.GetPlayerCameraManager` 0)))) false false)
  (`/Engine/EditorBlueprintResources/StandardMacros.IsValid` _returnvalue
    (:`Is Valid`
      (if (<= _returnvalue_2 (`self.ChaseRange`))
        (`self.Sync_StateIdx` true true 1)
        (if (<= _returnvalue_2 (`self.AttackRange`))
          (`self.Sync_bCanAttack` true true true)
          (else
            (`self.Sync_bCanAttack` true true :!label _label)))
        (else
          (`self.Sync_StateIdx` true true)
          (goto _label)))
      (if (<= (`self.HP`) 0.0)
        (`self.Sync_bIsDead` true true true)
        (set `CharacterMovementComponent.GravityScale` 0.0 (`self.CharacterMovement`))
        (`PrimitiveComponent.SetCollisionEnabled` (`self.CapsuleComponent`) "NoCollision")
        (bind _asplayer_character (cast `PlayerCharacter` (`GameplayStatics.GetPlayerCharacter` 0)))
        (bind _curenemynum (`PlayerCharacter.CurEnemyNum` _asplayer_character))
        (if (>= _curenemynum 1)
          (set `PlayerCharacter.CurEnemyNum` (- _curenemynum 1) _asplayer_character))
        (`KismetSystemLibrary.Delay` 4.0)
        (`self.K2_DestroyActor`)))))

(event `self.PawnSensing.OnSeePawn`
  (params (Pawn :type "Pawn Object Reference"))
  (`self.Sync_StateIdx` true true 1)
  (`self.SetMaxWalkSpeed` 450.0))

(event `self.DecreaseHP`
  (params (Value :type "Float (single-precision)"))
  (bind _output_get (set `self.HP` (- (`self.HP`) Value)))
  (`ProgressBar.SetPercent` (`self.Health PBar`) (/ _output_get (`self.MaxHP`)))
  (`self.Sync_StateIdx` true true 1))

(fn `MagicalLeaf`
  (for _array_element (`self.Leaves`)
    (bind _returnvalue (`SceneComponent.K2_GetComponentLocation` _array_element))
    (bind (_returnvalue_x _returnvalue_y) (`KismetMathLibrary.BreakVector` (- _returnvalue (`SceneComponent.K2_GetComponentLocation` (`self.Mesh`)))))
    (`|SpawnActorFromClass` "/Game/_shuby/Groot/BP_LeafBullet.BP_LeafBullet_C" (`KismetMathLibrary.MakeTransform` _returnvalue (`KismetMathLibrary.MakeRotFromX` (`KismetMathLibrary.Normal` (`KismetMathLibrary.MakeVector` _returnvalue_x _returnvalue_y) 1.0)) (`KismetMathLibrary.MakeVector` 0.4 0.4 0.4)) "AlwaysSpawn" "MultiplyWithRoot" null null)))

(fn `SetMaxWalkSpeed`
  (params (Speed :type "Float (double-precision)"))
  (set `CharacterMovementComponent.MaxWalkSpeed` Speed (`self.CharacterMovement`)))

(fn `Sync_bCanAttack`
  (params (ABP :type Boolean) (BBD :type Boolean) (Data :type Boolean))
  (bind _returnvalue (`AIBlueprintHelperLibrary.GetBlackboard` (`AIBlueprintHelperLibrary.GetAIController` self)))
  (`|ExecutionSequence`
    (:`then_0`
      (if ABP
        (bind _asabp_groot (cast `/Game/_shuby/Groot/ABP_Groot` (`SkeletalMeshComponent.GetAnimInstance` (`self.Mesh`))))
        (set `EnemyAnim.bAnimAttack` Data _asabp_groot)))
    (:`then_1`
      (if BBD
        (`/Engine/EditorBlueprintResources/StandardMacros.IsValid` _returnvalue
          (:`Is Valid`
            (`BlackboardComponent.SetValueAsBool` _returnvalue "bCanAttack" Data)))))))

(fn `Sync_bIsDead`
  (params (ABP :type Boolean) (BBD :type Boolean) (Data :type Boolean))
  (bind _returnvalue (`AIBlueprintHelperLibrary.GetBlackboard` (`AIBlueprintHelperLibrary.GetAIController` self)))
  (`|ExecutionSequence`
    (:`then_0`
      (if ABP
        (bind _asabp_groot (cast `/Game/_shuby/Groot/ABP_Groot` (`SkeletalMeshComponent.GetAnimInstance` (`self.Mesh`))))
        (set `EnemyAnim.bAnimDead` Data _asabp_groot)))
    (:`then_1`
      (if BBD
        (`/Engine/EditorBlueprintResources/StandardMacros.IsValid` _returnvalue
          (:`Is Valid`
            (`BlackboardComponent.SetValueAsBool` _returnvalue "bIsDead" Data)))))))

(fn `Sync_StateIdx`
  (params (ABP :type Boolean) (BBD :type Boolean) (Data :type Integer))
  (bind _returnvalue (`AIBlueprintHelperLibrary.GetBlackboard` (`AIBlueprintHelperLibrary.GetAIController` self)))
  (`|ExecutionSequence`
    (:`then_0`
      (if ABP
        (bind _asabp_groot (cast `/Game/_shuby/Groot/ABP_Groot` (`SkeletalMeshComponent.GetAnimInstance` (`self.Mesh`))))
        (set `EnemyAnim.AnimStateIdx` Data _asabp_groot)))
    (:`then_1`
      (if BBD
        (`/Engine/EditorBlueprintResources/StandardMacros.IsValid` _returnvalue
          (:`Is Valid`
            (`BlackboardComponent.SetValueAsInt` _returnvalue "StateIdx" Data)))))
    (:`then_2`
      (`self.SetMaxWalkSpeed` (`KismetMathLibrary.Conv_IntToDouble` (+ (* Data 250) 200))))))

(fn `UserConstructionScript`)