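; BP_LeafBullet is Groot's leaf bullet actor, which triggers a hit reaction on the player characters it overlaps.
; On overlap with a PlayerCharacter, it activates that character's abilities tagged State.Hit.Groot through the Ability System Component.
; It then activates its Niagara effect, hides both cone meshes and disables collision before a delayed self-destroy.
; A separate BeginPlay timer caps its lifetime at a few seconds.
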(event `self.ReceiveBeginPlay`
  (`KismetSystemLibrary.Delay` 3.0)
  (`self.K2_DestroyActor`))

(event `self.ReceiveActorBeginOverlap`
  (params (OtherActor :type "Actor Object Reference"))
  (bind _asplayer_character (cast `PlayerCharacter` OtherActor))
  (`AbilitySystemComponent.TryActivateAbilitiesByTag` (`AbilitySystemBlueprintLibrary.GetAbilitySystemComponent` _asplayer_character) (`BlueprintGameplayTagLibrary.MakeGameplayTagContainerFromTag` (struct :`TagName` "State.Hit.Groot")) true)
  (`ActorComponent.Activate` (`self.Niagara`) false)
  (`SceneComponent.SetVisibility` (`self.Cone`) false false)
  (`SceneComponent.SetVisibility` (`self.Cone1`) false false)
  (`self.SetActorEnableCollision` false)
  (`KismetSystemLibrary.Delay` 2.0)
  (`self.K2_DestroyActor`))

(fn `UserConstructionScript`)