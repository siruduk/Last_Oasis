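; Player controller for a 3D main menu, where clicking in-world signs starts the game or quits.
; On BeginPlay it enables the cursor, caches the level's CineCameraActor and shows WBP_MainUI.
; Every Tick and left click trace from that camera along the deprojected mouse direction, keeping the last valid hit actor.
; Clicking with BP_Sign1 stored fades the UI, then opens GameMap after a delay; BP_Sign2 quits.
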(event `self.ReceiveBeginPlay`
  (set `self.bShowMouseCursor` true)
  (set `self.bEnableClickEvents` true)
  (set `self.bEnableMouseOverEvents` true)
  (`WidgetBlueprintLibrary.SetInputMode_GameAndUIEx` self null "DoNotLock" false)
  (bind _returnvalue (`GameplayStatics.GetActorOfClass` "/Script/CinematicCamera.CineCameraActor"))
  (set `self.CineCamera` _returnvalue)
  (bind _returnvalue_2 (`|CreateWidget` "/Game/_shuby/UIs/WBP_MainUI.WBP_MainUI_C"))
  (bind _output_get (set `self.MainUI` _returnvalue_2))
  (`UserWidget.AddToViewport` _returnvalue_2 0)
  (`UserWidget.AddToViewport` _output_get 0))

(event `self.ReceiveTick`
  (params (DeltaSeconds :type "Float (single-precision)"))
  (`self.LineTrace`))

(event `Key|LeftMouseButton`
  (params (Key :type "Key Structure"))
  (bind _hitactor (`self.HitActor`))
  (:`Pressed`
    (`self.LineTrace`)
    (cast `/Game/_shuby/Main/BP_Sign1` _hitactor
      (:`then`
        (`/Game/_shuby/UIs/WBP_MainUI.Fade` (`self.MainUI`))
        (`KismetSystemLibrary.Delay` 3.0)
        (`GameplayStatics.OpenLevel` "GameMap"))
      (:`CastFailed`
        (cast `/Game/_shuby/Main/BP_Sign2` _hitactor)
        (`KismetSystemLibrary.QuitGame` null "Quit")))))

(fn `LineTrace`
  (bind _returnvalue (`self.K2_GetActorLocation` (`self.CineCamera`)))
  (bind _returnvalue_2 (`WidgetLayoutLibrary.GetMousePositionOnPlatform`))
  (bind (_returnvalue_x _returnvalue_y _returnvalue_z) (`KismetMathLibrary.BreakVector` (`KismetMathLibrary.Normal` (`.WorldDirection` (`GameplayStatics.DeprojectScreenToWorld` self _returnvalue_2)) 1.0)))
  (bind _outhit (`KismetSystemLibrary.LineTraceSingle` :`Start` _returnvalue :`End` (+ _returnvalue (* (`KismetMathLibrary.MakeVector` _returnvalue_x _returnvalue_y _returnvalue_z) (`self.TraceDirection`))) :`TraceChannel` "TraceTypeQuery1" :`DrawTime` 20.0))
  (bind (_bblockinghit _binitialoverlap _time _distance _location _impactpoint _normal _impactnormal _physmat _hitactor) (`GameplayStatics.BreakHitResult` _outhit))
  (`/Engine/EditorBlueprintResources/StandardMacros.IsValid` _hitactor
    (:`Is Valid`
      (set `self.HitActor` _hitactor))))

(fn `UserConstructionScript`)